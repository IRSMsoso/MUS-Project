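; BP_Sun is a procedural-mesh sun that pulses to a hard-coded music track as an audio visualizer.
; Each tick it samples the track's frequency spectrum at game time, maps bins by vertex angle, and scales base vertices with clamped, interpolated motion.
; SetProgress drives the SunLight parameter of its dynamic material through a progress curve.
; Min/Max tracking and unwired nodes are debug leftovers.
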(event EventBeginPlay
  (bind _returnvalue (Rendering|Material|CreateDynamicMaterialInstance (Variables|Default|GetProcMesh) 0 "/Game/Main/Materials/SunM.SunM" "None" :!class /Script/Engine.PrimitiveComponent))
  (Variables|Default|SetSun%20Dynamic%20Instance _returnvalue))

(event Collision|EventActorBeginOverlap
  (params (OtherActor :type Actor%20Object%20Reference)))

(event EventTick
  (params (DeltaSeconds :type Float%20%28single-precision%29))
  (bind _tempvertices (Variables|Default|GetTempVertices))
  (bind _outspectrum (Class|SoundVisualizationStatics|CalculateFrequencySpectrum "/Game/Main/Sound/Kavinsky_-_Nightcall__Drive_Original_Movie_Soundtrack___Official_Audio_-MV_3Dpw-BRY.Kavinsky_-_Nightcall__Drive_Original_Movie_Soundtrack___Official_Audio_-MV_3Dpw-BRY" 0 (Utilities|Time|GetGameTimeinSeconds) 0.08 20))
  (Variables|Default|SetPrevVerts _tempvertices)
  (Utilities|Array|Clear _tempvertices)
  (for (_array_element _array_index) (Variables|Default|GetSunVertices)
    (Utilities|Array|Add (Variables|Default|GetTempVertices) (Math|Interpolation|VInterpTo (Utilities|Array|Get(acopy) (Variables|Default|GetPrevVerts) _array_index) (Math|Vector|MakeVector (.x (* _array_element (Math|Float|Max(Float) (Math|Float|Min(Float) (* (Utilities|Array|Get(acopy) _outspectrum (Math|Integer|Max(Integer) (Math|Integer|Min(Integer) (Math|Float|Floor (* (Utilities|Array|Length _outspectrum) (+ (/ (Math|Trig|Atan(Degrees) (/ (.Y (Math|Vector|BreakVector _array_element)) (.X (Math|Vector|BreakVector _array_element)))) (Math|Trig|GetPI)) 0.5))) (- (Utilities|Array|Length _outspectrum) 1)))) 0.05) 2.5) 0.5))) (.y (* _array_element (Math|Float|Max(Float) (Math|Float|Min(Float) (* (Utilities|Array|Get(acopy) _outspectrum (Math|Integer|Max(Integer) (Math|Integer|Min(Integer) (Math|Float|Floor (* (Utilities|Array|Length _outspectrum) (+ (/ (Math|Trig|Atan(Degrees) (/ (.Y (Math|Vector|BreakVector _array_element)) (.X (Math|Vector|BreakVector _array_element)))) (Math|Trig|GetPI)) 0.5))) (- (Utilities|Array|Length _outspectrum) 1)))) 0.05) 2.5) 0.5))) (.Z (Math|Vector|BreakVector _array_element))) DeltaSeconds 5.0)))
  (Class|ProceduralMeshComponent|UpdateMeshSectionLinearColor (Variables|Default|GetProcMesh) 0 (Variables|Default|GetTempVertices))
  (for _array_element_2 (Variables|Default|Gettest)
    (Utilities|FlowControl|Sequence
      (:then_0
        (if (< _array_element_2 (Variables|Default|GetMin))
          (Variables|Default|SetMin _array_element_2)))
      (:then_1
        (if (> _array_element_2 (Variables|Default|GetMax))
          (Variables|Default|SetMax _array_element_2))))))

(fn ConstructionScript)

(fn SetProgress
  (params (Progress :type Float%20%28single-precision%29))
  (Rendering|Material|SetScalarParameterValue (Variables|Default|GetSun%20Dynamic%20Instance) "SunLight" (Math|Curves|GetFloatValue (Variables|Default|GetSunlight%20Progress%20Curve) Progress) :!class /Script/Engine.MaterialInstanceDynamic))