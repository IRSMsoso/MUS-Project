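; RockBP is an audio visualizer actor that deforms a procedural mesh grid from the frequency spectrum of a hardcoded Nightcall music track.
; Each Tick samples a short spectrum window at the current game time and pushes it into a row buffer capped at GridY, forming a scrolling history.
; The buffered values drive vertex heights before the mesh section updates.
; The construction script only assigns a walnut material, and no mesh creation appears here.
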(event EventBeginPlay)

(event EventTick
  (params (DeltaSeconds :type Float%20%28single-precision%29))
  (bind _spectrumrowbuffer (Variables|Default|GetSpectrumRowBuffer))
  (bind _gridx (Variables|Default|GetGridX))
  (bind _vertices (Variables|Default|GetVertices))
  (bind _outspectrum (Class|SoundVisualizationStatics|CalculateFrequencySpectrum "/Game/Main/Sound/Kavinsky_-_Nightcall__Drive_Original_Movie_Soundtrack___Official_Audio_-MV_3Dpw-BRY.Kavinsky_-_Nightcall__Drive_Original_Movie_Soundtrack___Official_Audio_-MV_3Dpw-BRY" 0 (Utilities|Time|GetGameTimeinSeconds) 0.08 (Variables|Default|GetGridX)))
  (Utilities|Array|Insert _spectrumrowbuffer (Utilities|Struct|MakeSpectrumRow _outspectrum))
  (Utilities|Array|Resize _spectrumrowbuffer (Variables|Default|GetGridY))
  (for _index (range 0 (Variables|Default|GetGridY))
    (for _index_2 (range 0 _gridx)
      (Utilities|Array|SetArrayElem _vertices (+ (* _index _gridx) _index_2) (Math|Vector|MakeVector (.x (Utilities|Array|Get(acopy) _vertices (+ (* _index _gridx) _index_2))) (.y (Utilities|Array|Get(acopy) _vertices (+ (* _index _gridx) _index_2))) (* (Utilities|Array|Get(acopy) (Utilities|Struct|BreakSpectrumRow (Utilities|Array|Get(acopy) (Variables|Default|GetSpectrumRowBuffer) _index)) _index_2) 1e+01)))))
  (Class|ProceduralMeshComponent|UpdateMeshSectionLinearColor (Variables|Default|GetProcMesh) 0 (Variables|Default|GetVertices)))

(fn ConstructionScript
  (Rendering|Material|SetMaterial (Variables|Default|GetProcMesh) 0 "/Game/StarterContent/Materials/M_Wood_Floor_Walnut_Polished.M_Wood_Floor_Walnut_Polished"))