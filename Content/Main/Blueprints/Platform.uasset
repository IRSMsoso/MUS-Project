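; Music-reactive platform actor that travels along X as the Kavinsky "Nightcall" track plays and passes playback progress to its child BP_Sun.
; The audio envelope runs through two curves to pulse the emissive strength of a dynamic vapor-grid material each tick.
; BeginPlay also overrides the static mesh variable on the Tar Niagara system.
; An unconnected branch that would deform a procedural mesh from scrolling frequency spectrum rows never runs.
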(event OnAudioSingleEnvelopeValue(Kavinsky_-_Nightcall__Drive_Original_Movie_Soundtrack___Official_Audio_-MV_3Dpw-BRY)
  (params (PlayingSoundWave :type Sound%20Wave%20Object%20Reference) (EnvelopeValue :type Float%20%28single-precision%29))
  (Variables|Default|SetNormalized%20Amplitude (Math|Curves|GetFloatValue (Variables|Curves|GetNormalize%20Audio%20Curve) EnvelopeValue)))

(event OnAudioPlaybackPercent(Kavinsky_-_Nightcall__Drive_Original_Movie_Soundtrack___Official_Audio_-MV_3Dpw-BRY)
  (params (PlayingSoundWave :type Sound%20Wave%20Object%20Reference) (PlaybackPercent :type Float%20%28single-precision%29))
  (Transformation|SetActorLocation (Math|Vector|MakeVector (* PlaybackPercent 1.665e+04) 0.0 -1e+02) false false)
  (bind _asbp_sun (Utilities|Casting|CastToBP_Sun (Variables|/Script/Engine.ChildActorComponent|GetChildActor (Variables|Default|GetSun))))
  (Default|SetProgress _asbp_sun PlaybackPercent))

(event EventBeginPlay
  (bind _returnvalue (Rendering|Material|CreateDynamicMaterialInstance (Variables|Default|GetStaticMesh) 0 "/Game/Main/Materials/VaprGridInstance.VaprGridInstance" "DI_VaporGrid" :!class /Script/Engine.PrimitiveComponent))
  (Variables|Default|SetVaporGrid%20Dynamic%20Instance _returnvalue)
  (Class|NiagaraFunctionLibrary|OverrideSystemUserVariableStaticMeshComponent (Variables|Default|GetTar) "Static Mesh"))

(event Collision|EventActorBeginOverlap
  (params (OtherActor :type Actor%20Object%20Reference)))

(event EventTick
  (params (DeltaSeconds :type Float%20%28single-precision%29))
  (Rendering|Material|SetScalarParameterValue (Variables|Default|GetVaporGrid%20Dynamic%20Instance) "Emissive Amount" (Math|Curves|GetFloatValue (Variables|Curves|GetNormalized%20Amplitude%20To%20Emissive%20Strength%20Curve) (Variables|Default|GetNormalized%20Amplitude)) :!class /Script/Engine.MaterialInstanceDynamic))

(fn ConstructionScript)